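; BP_Spikezone is a hazard volume that damages characters while they overlap its box.
; Box begin and end overlap events add and remove overlapping Characters in a tracked array, ignoring other actor types.
; Each Tick applies DPS scaled by delta time to every tracked character, giving frame-rate-independent continuous damage with the zone as the damage causer.
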(event `self.ReceiveTick`
  (params (DeltaSeconds :type "Float (single-precision)"))
  (for _array_element (`self.Characters in spikes`)
    (`GameplayStatics.ApplyDamage` _array_element (* (`self.DPS`) DeltaSeconds) null self)))

(event `self.Box.OnComponentBeginOverlap`
  (params (OverlappedComponent :type "PrimitiveComponent Object Reference") (OtherActor :type "Actor Object Reference") (OtherComp :type "PrimitiveComponent Object Reference") (OtherBodyIndex :type Integer) (bFromSweep :type Boolean) (SweepResult :type "HitResult Structure (by ref)"))
  (bind _ascharacter (cast `Character` OtherActor))
  (`KismetArrayLibrary.Array_AddUnique` (`self.Characters in spikes`) _ascharacter))

(event `self.Box.OnComponentEndOverlap`
  (params (OverlappedComponent :type "PrimitiveComponent Object Reference") (OtherActor :type "Actor Object Reference") (OtherComp :type "PrimitiveComponent Object Reference") (OtherBodyIndex :type Integer))
  (bind _ascharacter (cast `Character` OtherActor))
  (`KismetArrayLibrary.Array_RemoveItem` (`self.Characters in spikes`) _ascharacter))

(fn `UserConstructionScript`)