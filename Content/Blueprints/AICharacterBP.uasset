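; AI character Blueprint that wanders the navmesh, reacts to sensed pawns and destroys itself when damage depletes its health.
; Tick moves toward TargetLocation; on arrival or failure, a short Delay precedes picking a random reachable point nearby.
; PawnSensing overrides that target with the navmesh-projected pawn location: fast when seen, slow when heard above HearingCutoff.
; Walk speed persists after sensing, and the KillVolume overlap event is empty.
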(event `self.ReceiveAnyDamage`
  (params (Damage :type "Float (single-precision)") (DamageType :type "DamageType Object Reference") (InstigatedBy :type "Controller Object Reference") (DamageCauser :type "Actor Object Reference"))
  (bind _output_get (set `self.Health` (- (`self.Health`) Damage)))
  (if (<= (`KismetMathLibrary.FTrunc` _output_get) 0)
    (`self.K2_DestroyActor`)))

(event `self.ReceiveBeginPlay`
  ;[1 1 1] Setting first destination
  (set `self.AI Controller` (`AIBlueprintHelperLibrary.GetAIController` self))
  (set `self.Target Location` (`self.K2_GetActorLocation`)))

(event `self.ReceiveTick`
  (params (DeltaSeconds :type "Float (single-precision)"))
  ;[1 1 1] AI Random movement
  (bind _returnvalue (`AIController.MoveToLocation` (`self.AI Controller`) (`self.Target Location`) -1.0 true true false true null true))
  (switch `EPathFollowingRequestResult` _returnvalue
    (:`Failed`
      _)
    (:`AlreadyAtGoal`
      _))
  (`KismetSystemLibrary.Delay` 2.5)
  (set `self.Target Location` (`NavigationSystemV1.K2_GetRandomReachablePointInRadius` (`self.Target Location`) (`self.Wonder Radius`) (`self.Nav Data`) null)))

(event `self.PawnSensing.OnSeePawn`
  (params (Pawn :type "Pawn Object Reference"))
  ;[1 1 1] AI Seeing player
  (set `CharacterMovementComponent.MaxWalkSpeed` 600.0 (`self.CharacterMovement`))
  (set `self.Target Location` (`NavigationSystemV1.K2_ProjectPointToNavigation` (`self.K2_GetActorLocation` Pawn) (`self.Nav Data`))))

(event `self.PawnSensing.OnHearNoise`
  (params (Instigator :type "Pawn Object Reference") (Location :type "Vector Structure (by ref)") (Volume :type "Float (single-precision)"))
  ;[1 1 1] AI Hearing player
  (if (>= Volume (`self.Hearing Cutoff`))
    (set `CharacterMovementComponent.MaxWalkSpeed` 100.0 (`self.CharacterMovement`))
    (set `self.Target Location` (`NavigationSystemV1.K2_ProjectPointToNavigation` (`self.K2_GetActorLocation` Instigator) (`self.Nav Data`)))))

(event `self.Kill Volume.OnComponentBeginOverlap`
  (params (OverlappedComponent :type "PrimitiveComponent Object Reference") (OtherActor :type "Actor Object Reference") (OtherComp :type "PrimitiveComponent Object Reference") (OtherBodyIndex :type Integer) (bFromSweep :type Boolean) (SweepResult :type "HitResult Structure (by ref)")))

(fn `UserConstructionScript`)