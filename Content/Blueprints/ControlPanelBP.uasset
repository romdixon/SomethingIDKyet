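; ControlPanelBP is a control panel actor that lets the player unlock a linked door.
; Overlapping it shows tutorial text on a referenced TextRender actor and enables player input on the panel.
; Releasing E clears the door's IsLocked flag and shows unlocked text.
; Leaving the overlap restores the exit text, also set on BeginPlay, and disables input.
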(event `self.ReceiveBeginPlay`
  ;[1 1 1] On Begin play Set to empty text
  (`TextRenderComponent.K2_SetText` (`TextRenderActor.TextRender` (`self.Text Render ActorTo Change`)) (`KismetTextLibrary.Conv_StringToText` (`self.Exit Text`))))

(event `self.ReceiveActorBeginOverlap`
  (params (OtherActor :type "Actor Object Reference"))
  ;[1 1 1] On Actor begin overlap set text to tutorial text and listen for keyboard imput
  (`TextRenderComponent.K2_SetText` (`TextRenderActor.TextRender` (`self.Text Render ActorTo Change`)) (`KismetTextLibrary.Conv_StringToText` (`self.Tutorial Text`)))
  (`self.EnableInput` self (`GameplayStatics.GetPlayerController` 0)))

(event `self.ReceiveActorEndOverlap`
  (params (OtherActor :type "Actor Object Reference"))
  ;[1 1 1] On Actor end overlap set text to exit text and stop listening for keyboard imput
  (`TextRenderComponent.K2_SetText` (`TextRenderActor.TextRender` (`self.Text Render ActorTo Change`)) (`KismetTextLibrary.Conv_StringToText` (`self.Exit Text`)))
  (`self.DisableInput` self (`GameplayStatics.GetPlayerController` 0)))

(event `Key|E`
  (params (Key :type "Key Structure"))
  ;[1 1 1] One E Unlock the door And provide feedback
  (:`Released`
    (set `/Game/Blueprints/MovingDoorBP.IsLocked` false (`self.Door To unlock`))
    (`TextRenderComponent.K2_SetText` (`TextRenderActor.TextRender` (`self.Text Render ActorTo Change`)) (`KismetTextLibrary.Conv_StringToText` (`self.Unlocked Text`)))))

(fn `UserConstructionScript`)