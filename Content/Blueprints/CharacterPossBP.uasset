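; A trigger actor that lets the player swap control between a Human and a Robot pawn as part of a door puzzle.
; Input is disabled at begin play and enabled only during an overlap, so E works inside the trigger.
; E possesses the Robot if the Human is player-controlled; otherwise it repossesses the Human and plays the Puzzle2Movingdoor sequence, pausing at its end.
; Each press then disables the trigger's input.
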(event `self.ReceiveActorEndOverlap`
  (params (OtherActor :type "Actor Object Reference"))
  ;[1 1 1] Once player has left trigger disable input
  (`self.DisableInput` (`GameplayStatics.GetPlayerController` 0) :!label _label))

(event `self.ReceiveBeginPlay`
  ;[1 1 1] Once player has left trigger disable input
  (goto _label))

(event `self.ReceiveActorBeginOverlap`
  (params (OtherActor :type "Actor Object Reference"))
  ;[1 1 1] When player enters trigger enable enput only after E is pressed
  (`self.EnableInput` (`GameplayStatics.GetPlayerController` 0)))

(event `Key|E`
  (params (Key :type "Key Structure"))
  (bind _returnvalue (`GameplayStatics.GetPlayerController` 0))
  ;[1 1 1] Once the player has entered the trigger and has pressed E you will control the robot player needs to move him into the next trigger and press E in order to regain control of the player once this happens a sequence of a door opening will play
  (:`Pressed`
    (if (`Pawn.IsPlayerControlled` (`self.Human`))
      (`Controller.Possess` _returnvalue (`self.Robot`))
      (else
        (`Controller.Possess` _returnvalue (`self.Human`))
        (bind _outactor (`LevelSequencePlayer.CreateLevelSequencePlayer` "/Game/Sequences/Puzzle2Movingdoor.Puzzle2Movingdoor" (make `MovieSceneSequencePlaybackSettings` false (struct) 1.0 0.0 false false false false false false false true)))
        (`MovieSceneSequencePlayer.Play` (`LevelSequenceActor.SequencePlayer` _outactor))))
    (`self.DisableInput` null)))

(fn `UserConstructionScript`)