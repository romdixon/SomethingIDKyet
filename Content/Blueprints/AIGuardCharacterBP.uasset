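; AI guard character that patrols waypoints, chases seen pawns, investigates noises and destroys the player on kill-volume overlap.
; Tick drives MoveToLocation toward a navmesh-projected target, advancing waypoints after a delay when the goal is reached or fails.
; PawnSensing overrides target and speed for sightings or loud noises, with DoOnce sound cues that re-arm when patrol resumes.
; Any damage reduces health, destroying the guard when it runs out.
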(event `self.ReceiveAnyDamage`
  (params (Damage :type "Float (single-precision)") (DamageType :type "DamageType Object Reference") (InstigatedBy :type "Controller Object Reference") (DamageCauser :type "Actor Object Reference"))
  ;[1 1 1] Kills AI after time
  (bind _output_get (set `self.Health` (- (`self.Health`) Damage)))
  (if (<= (`KismetMathLibrary.FTrunc` _output_get) 0)
    (`self.K2_DestroyActor`)))

(event `self.ReceiveBeginPlay`
  ;[1 1 1] First waypoint
  (set `self.AI Controller` (`AIBlueprintHelperLibrary.GetAIController` self))
  (set `self.Target Location` (`NavigationSystemV1.K2_ProjectPointToNavigation` (`self.K2_GetActorLocation`) (`self.Nav Data`)))
  (set `CharacterMovementComponent.MaxWalkSpeed` (`self.Walking speed`) (`self.CharacterMovement`)))

(event `self.ReceiveTick`
  (params (DeltaSeconds :type "Float (single-precision)"))
  ;[1 1 1] Moving through the waypoints
  (bind _returnvalue (`AIController.MoveToLocation` (`self.AI Controller`) (`self.Target Location`) -1.0 true true false true null true))
  (switch `EPathFollowingRequestResult` _returnvalue
    (:`Failed`
      _)
    (:`AlreadyAtGoal`
      _))
  (`KismetSystemLibrary.Delay` 0.5)
  (`/Engine/EditorBlueprintResources/StandardMacros.IncrementInt` (`self.Current Waypoint`)
    (:`  `
      (if (<= (`self.Current Waypoint`) (`KismetArrayLibrary.Array_Length` (`self.Waypoints`)))
        (set `self.Target Location` (`NavigationSystemV1.K2_ProjectPointToNavigation` (`self.K2_GetActorLocation` (`|GetArrayItem` (`self.Waypoints`) (`self.Current Waypoint`))) (`self.Nav Data`)))
        (set `CharacterMovementComponent.MaxWalkSpeed` (`self.Walking speed`) (`self.CharacterMovement`))
        (`|ExecutionSequence`
          (:`then_0`
            (goto _label :!via `Reset`))
          (:`then_1`
            (goto _label_2 :!via `Reset`)))
        (else
          (set `self.Current Waypoint` 0))))))

(event `self.Kill Volume.OnComponentBeginOverlap`
  (params (OverlappedComponent :type "PrimitiveComponent Object Reference") (OtherActor :type "Actor Object Reference") (OtherComp :type "PrimitiveComponent Object Reference") (OtherBodyIndex :type Integer) (bFromSweep :type Boolean) (SweepResult :type "HitResult Structure (by ref)"))
  ;[1 1 1] If enter killV then kill(Destroy)
  (if (== OtherActor (`GameplayStatics.GetPlayerPawn` 0))
    (`self.K2_DestroyActor` OtherActor)))

(event `self.PawnSensing.OnSeePawn`
  (params (Pawn :type "Pawn Object Reference"))
  ;[1 1 1] AI Seeing player
  (set `CharacterMovementComponent.MaxWalkSpeed` (`self.Running speed`) (`self.CharacterMovement`))
  (set `self.Target Location` (`NavigationSystemV1.K2_ProjectPointToNavigation` (`self.K2_GetActorLocation` Pawn) (`self.Nav Data`)))
  ;[1 1 1] Play sound once until patrol again
  (`/Engine/EditorBlueprintResources/StandardMacros.DoOnce` false :!label _label
    (:`Completed`
      (`GameplayStatics.PlaySoundAtLocation` "/Engine/VREditor/Sounds/UI/Camera_Shutter.Camera_Shutter" (`self.K2_GetActorLocation`) (struct) 1.0 1.0 0.0 null null null))))

(event `self.PawnSensing.OnHearNoise`
  (params (Instigator :type "Pawn Object Reference") (Location :type "Vector Structure (by ref)") (Volume :type "Float (single-precision)"))
  ;[1 1 1] AI Hearing player
  (if (>= Volume (`self.Hearing Cuttoff`))
    (set `CharacterMovementComponent.MaxWalkSpeed` 100.0 (`self.CharacterMovement`))
    (set `self.Target Location` (`NavigationSystemV1.K2_ProjectPointToNavigation` (`self.K2_GetActorLocation` Instigator) (`self.Nav Data`)))
    ;[1 1 1] Play sound once until patrol again
    (`/Engine/EditorBlueprintResources/StandardMacros.DoOnce` false :!label _label_2
      (:`Completed`
        (`GameplayStatics.PlaySoundAtLocation` "/Engine/VREditor/Sounds/VR_confirm.VR_confirm" (`self.K2_GetActorLocation`) (struct) 1.0 1.0 0.0 null null null)))))

(fn `UserConstructionScript`)