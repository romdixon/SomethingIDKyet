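; Control panel screen actor that displays one of three camera views by swapping the material on its static mesh.
; Every Tick it switches on CameraNumberToShow and applies the matching entry from the Materials array to element 0.
; Any value outside 0 to 2 resets the number to 0, so the first view shows on a later tick.
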(event `self.ReceiveTick`
  (params (DeltaSeconds :type "Float (single-precision)"))
  (switch `int` (`self.Camera Number to show`)
    (:`Default`
      (set `self.Camera Number to show` 0))
    (:`0`
      ;[1 1 1] Set Material to 0
      (`PrimitiveComponent.SetMaterial` (`self.StaticMeshComponent`) 0 (`|GetArrayItem` (`self.Materials`))))
    (:`1`
      ;[1 1 1] Set Material to 1
      (`PrimitiveComponent.SetMaterial` (`self.StaticMeshComponent`) 0 (`|GetArrayItem` (`self.Materials`) 1)))
    (:`2`
      ;[1 1 1] Set Material 2
      (`PrimitiveComponent.SetMaterial` (`self.StaticMeshComponent`) 0 (`|GetArrayItem` (`self.Materials`) 2)))))

(fn `UserConstructionScript`)