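; TutorialTextBP is an overlap-triggered actor that shows tutorial text on a referenced TextRenderActor.
; Beginning an overlap sets that actor's text to TutorialText, and ending it swaps to ExitText, with no filter on the overlapping actor.
; An unconnected leftover chain would create and play the Doorsequences level sequence, but it never runs.
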(event `self.ReceiveActorBeginOverlap`
  (params (OtherActor :type "Actor Object Reference"))
  (`TextRenderComponent.K2_SetText` (`TextRenderActor.TextRender` (`self.Text Render ActorTo Change`)) (`KismetTextLibrary.Conv_StringToText` (`self.Tutorial Text`))))

(event `self.ReceiveActorEndOverlap`
  (params (OtherActor :type "Actor Object Reference"))
  (`TextRenderComponent.K2_SetText` (`TextRenderActor.TextRender` (`self.Text Render ActorTo Change`)) (`KismetTextLibrary.Conv_StringToText` (`self.Exit Text`))))

(fn `UserConstructionScript`)