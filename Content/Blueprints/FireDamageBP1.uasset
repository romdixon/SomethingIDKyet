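; Fire hazard actor that deals continuous damage to player characters standing inside its box volume.
; Box overlap events add and remove ThirdPersonCharacter actors in the CharacterInFire array.
; Tick applies DPS scaled by delta time to every tracked character, so damage per second stays frame-rate independent.
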(event `self.ReceiveTick`
  (params (DeltaSeconds :type "Float (single-precision)"))
  (for _array_element (`self.Character in Fire`)
    (`GameplayStatics.ApplyDamage` _array_element (* (`self.DPS`) DeltaSeconds) null self)))

(event `self.Box.OnComponentBeginOverlap`
  (params (OverlappedComponent :type "PrimitiveComponent Object Reference") (OtherActor :type "Actor Object Reference") (OtherComp :type "PrimitiveComponent Object Reference") (OtherBodyIndex :type Integer) (bFromSweep :type Boolean) (SweepResult :type "HitResult Structure (by ref)"))
  (bind _asthird_person_character (cast `/Game/ThirdPersonBP/Blueprints/ThirdPersonCharacter` OtherActor))
  (`KismetArrayLibrary.Array_Add` (`self.Character in Fire`) _asthird_person_character))

(event `self.Box.OnComponentEndOverlap`
  (params (OverlappedComponent :type "PrimitiveComponent Object Reference") (OtherActor :type "Actor Object Reference") (OtherComp :type "PrimitiveComponent Object Reference") (OtherBodyIndex :type Integer))
  (bind _asthird_person_character (cast `/Game/ThirdPersonBP/Blueprints/ThirdPersonCharacter` OtherActor))
  (`KismetArrayLibrary.Array_RemoveItem` (`self.Character in Fire`) _asthird_person_character))

(fn `UserConstructionScript`)