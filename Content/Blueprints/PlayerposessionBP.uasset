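; PlayerposessionBP is an interaction actor that swaps player possession between a Human and a Robot pawn.
; Its input is disabled at BeginPlay, enabled for player controller 0 when any actor begins overlapping it, and disabled again when an overlap ends.
; Pressing E possesses the Robot if the Human is player-controlled, otherwise the Human, then calls DisableInput.
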(event `self.ReceiveActorEndOverlap`
  (params (OtherActor :type "Actor Object Reference"))
  (`self.DisableInput` (`GameplayStatics.GetPlayerController` 0) :!label _label))

(event `self.ReceiveBeginPlay`
  (goto _label))

(event `self.ReceiveActorBeginOverlap`
  (params (OtherActor :type "Actor Object Reference"))
  (`self.EnableInput` (`GameplayStatics.GetPlayerController` 0)))

(event `Key|E`
  (params (Key :type "Key Structure"))
  (bind _returnvalue (`GameplayStatics.GetPlayerController` 0))
  (:`Pressed`
    (if (`Pawn.IsPlayerControlled` (`self.Human`))
      (`Controller.Possess` _returnvalue (`self.Robot`))
      (else
        (`Controller.Possess` _returnvalue (`self.Human`))))
    (`self.DisableInput` null)))

(fn `UserConstructionScript`)