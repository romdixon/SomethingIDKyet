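; KnockBP is an interactable actor that lets the player make a knock to draw AI characters to their position.
; It enables its own input only while the player pawn overlaps it, disabling it on BeginPlay and when the overlap ends.
; Pressing E sets TargetLocation on every AICharacterBP in the level to the player pawn's current location, with no distance check.
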(event `self.ReceiveBeginPlay`
  (`self.DisableInput` (`GameplayStatics.GetPlayerController` 0) :!label _label))

(event `self.ReceiveActorEndOverlap`
  (params (OtherActor :type "Actor Object Reference"))
  (if (== OtherActor (`GameplayStatics.GetPlayerPawn` 0))
    (goto _label)))

(event `self.ReceiveActorBeginOverlap`
  (params (OtherActor :type "Actor Object Reference"))
  (if (== OtherActor (`GameplayStatics.GetPlayerPawn` 0))
    (`self.EnableInput` (`GameplayStatics.GetPlayerController` 0))))

(event `Key|E`
  (params (Key :type "Key Structure"))
  (:`Pressed`
    (bind _outactors (`GameplayStatics.GetAllActorsOfClass` "/Game/Blueprints/AICharacterBP.AICharacterBP_C"))
    (for _array_element _outactors
      (set `/Game/Blueprints/AICharacterBP.Target Location` (`self.K2_GetActorLocation` (`GameplayStatics.GetPlayerPawn` 0)) _array_element))))

(fn `UserConstructionScript`)