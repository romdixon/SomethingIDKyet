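; Launch pad actor that throws any Character overlapping its box upward at LaunchZ and plays a low-pitched steam sound.
; The construction script creates a dynamic material instance on the mesh from the Color and Intensity variables.
; On BeginPlay, a timeline animates that material's Intensity parameter to flash the pad.
; The node that would apply FlashRate to the timeline is unconnected, so that variable has no effect on the flashing.
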(event `self.ReceiveBeginPlay`
  (`self.Start Flashing`))

(event `Start Flashing`
  (bind (_direction _0_to_1) (`Timeline|Flashing Timeline`)
    (:`Update`
      (`MaterialInstanceDynamic.SetScalarParameterValue` (`self.MaterialRef`) "Intensity" (`KismetMathLibrary.Lerp` 1.0 10.0 _0_to_1)))))

(event `self.Box.OnComponentBeginOverlap`
  (params (OverlappedComponent :type "PrimitiveComponent Object Reference") (OtherActor :type "Actor Object Reference") (OtherComp :type "PrimitiveComponent Object Reference") (OtherBodyIndex :type Integer) (bFromSweep :type Boolean) (SweepResult :type "HitResult Structure (by ref)"))
  (bind _ascharacter (cast `Character` OtherActor))
  (`Character.LaunchCharacter` _ascharacter (`KismetMathLibrary.MakeVector` 0.0 0.0 (`self.LaunchZ`)) false false)
  (`GameplayStatics.SpawnSoundAtLocation` "/Game/StarterContent/Audio/Steam01_Cue.Steam01_Cue" (`self.K2_GetActorLocation`) (struct) 1.0 0.25 0.0 null null))

(fn `UserConstructionScript`
  (bind _returnvalue (`PrimitiveComponent.CreateDynamicMaterialInstance` (`self.StaticMesh`) 0 "/Game/Launchpad/LaunchPadMaterial.LaunchPadMaterial" "None"))
  (set `self.MaterialRef` _returnvalue)
  (`MaterialInstanceDynamic.SetVectorParameterValue` _returnvalue "Color" (`self.Color`))
  (`MaterialInstanceDynamic.SetScalarParameterValue` _returnvalue "Intensity" (`self.Intensity`)))